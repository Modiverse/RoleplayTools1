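; Keypad Cracker player tool that activates a Keypad after the primary button is held on it for five seconds.
; The local client forwards button state and requests a server check each Tick.
; The server traces from the camera proxy, runs a timer that cancels on release or lost aim, then calls KeypadActivated.
; BeginPlay registers the tool, creates assist and progress bar widgets, and saves equipment-bar visibility.
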(event `self.ReceiveBeginPlay`
  (bind _basetoolsavegamebp (`self.BaseToolSaveGameBP`))
  ;[0.9593 1 0.1335] BEGIN PLAY EVENT
  (`/Game/CustomContent/UGC2289475071/KJModMacroLibrary.HandleClientServerLogic`
    (:`ClientLogic`
      ;;[1 1 1] If local controlled; init once..
      (`self.IsLocallyControlled`
        (:`Local`
          (`self.RegisterToolLocally`)
          (`self.CreateAndShowToolsAssistinformation`)
          (bind _returnvalue (`|CreateWidget` "/Game/CustomContent/UGC2289475071/Blueprints/KeypadCracker/ProgressBarWidgetBP.ProgressBarWidgetBP_C" (`GameplayStatics.GetPlayerController` 0)))
          (set `self.ProgressBarWidgetBP` _returnvalue)
          (bind _returnvalue_2 (`self.LoadToolSettings` "KeypadCrackerBaseSettings"))
          (`KismetSystemLibrary.PrintString` "loaded tool settings")
          (`/Engine/EditorBlueprintResources/StandardMacros.IsValid` _returnvalue_2
            (:`Is Valid`
              (`KismetSystemLibrary.PrintString` "tool setting found")
              (bind _asbase_tool_save_game_bp (cast `/Game/CustomContent/UGC2289475071/Blueprints/BaseToolSaveGameBP` _returnvalue_2))
              (set `self.BaseToolSaveGameBP` _asbase_tool_save_game_bp))
            (:`Is Not Valid`
              (`KismetSystemLibrary.PrintString` "no tool settings found.- creating")
              (bind _returnvalue_3 (`GameplayStatics.CreateSaveGameObject` "/Game/CustomContent/UGC2289475071/Blueprints/BaseToolSaveGameBP.BaseToolSaveGameBP_C"))
              (set `self.BaseToolSaveGameBP` _returnvalue_3)))
          (set `/Game/CustomContent/UGC2289475071/Blueprints/BaseToolSaveGameBP.bVisibleOnEquipmentBar` true _basetoolsavegamebp)
          (`KismetSystemLibrary.PrintString` "set visiable on equipmentbar to true")
          (`self.SaveToolSettings` "KeypadCrackerBaseSettings" _basetoolsavegamebp))))))

(event `self.ReceiveTick`
  (params (DeltaSeconds :type "Float (single-precision)"))
  (bind _activatetimer (`self.ActivateTimer`))
  (bind _returnvalue (`KismetSystemLibrary.K2_GetTimerElapsedTimeHandle` _activatetimer))
  (`/Game/CustomContent/UGC2289475071/KJModMacroLibrary.HandleClientServerLogic`
    (:`ClientLogic`
      (`self.IsLocallyControlled`
        (:`Local`
          (`self.LookForKeypadToCrackServer`)
          (if (`KismetSystemLibrary.K2_IsTimerActiveHandle` _activatetimer)
            (`/Game/CustomContent/UGC2289475071/Blueprints/KeypadCracker/ProgressBarWidgetBP.UpdateProgress` (`self.ProgressBarWidgetBP`) (/ _returnvalue (+ _returnvalue (`KismetSystemLibrary.K2_GetTimerRemainingTimeHandle` _activatetimer))))))))))

(event `LookForKeypadToCrackServer`
  (bind _activatetimer (`self.ActivateTimer`))
  (bind _activatetimer_2 (`self.ActivateTimer`))
  (`/Game/CustomContent/UGC2289475071/KJModMacroLibrary.HandleClientServerLogic`
    (:`ServerLogic`
      (if (`self.Pressed`)
        (bind _returnvalue (`self.GetPawnRemoteCameraProxyComponent`))
        (bind _returnvalue_2 (`SceneComponent.K2_GetComponentLocation` _returnvalue))
        (bind (_outhit _returnvalue_3) (`KismetSystemLibrary.LineTraceSingle` _returnvalue_2 (+ _returnvalue_2 (* (`SceneComponent.GetForwardVector` _returnvalue) 500.0)) "TraceTypeQuery1" true (`|MakeArray` (`GameplayStatics.GetPlayerPawn` 0) :!type "Actor Object Reference"))) ; Look for keypad
        (if _returnvalue_3
          (bind _askeypad (cast `/Game/CustomContent/UGC2289475071/Blueprints/Keypad/Keypad` (`.HitActor` (`GameplayStatics.BreakHitResult` _outhit)))
            (:`then`
              (if (not (`KismetSystemLibrary.K2_IsTimerActiveHandle` (`self.ActivateTimer`)))
                (set `self.Keypad` _askeypad)
                (bind _returnvalue_4 (`KismetSystemLibrary.K2_SetTimer` null "ActivateKeypad" 5.0))
                (set `self.ActivateTimer` _returnvalue_4)
                (`self.ShowProgressBar`)))
            (:`CastFailed`
              (if (`KismetSystemLibrary.K2_IsValidTimerHandle` _activatetimer) :!label _label
                (`KismetSystemLibrary.K2_ClearAndInvalidateTimerHandle` _activatetimer)
                (`self.HideProgressBar`))))
          (else
            (goto _label)))
        (elif (`KismetSystemLibrary.K2_IsValidTimerHandle` _activatetimer_2)
          (`KismetSystemLibrary.K2_ClearAndInvalidateTimerHandle` _activatetimer_2)
          (`self.HideProgressBar`))))))

(event `KJModToolProxyInterface.ToolProxy_PrimaryMouseClick`
  (params (pressed :type Boolean))
  (`/Game/CustomContent/UGC2289475071/KJModMacroLibrary.HandleClientServerLogic`
    (:`ClientLogic`
      (`self.IsLocallyControlled`
        (:`Local`
          (`self.ToggledPressedOnServer` pressed))))))

(event `ToggledPressedOnServer`
  (params (Pressed :type Boolean))
  (set `self.Pressed` Pressed))

(event `PlayToolSoundFromServer`
  (`self.PlayToolSoundEffect` "ToolSpawnSound"))

(event `ShowProgressBar`
  (`UserWidget.AddToViewport` (`self.ProgressBarWidgetBP`) 0))

(event `HideProgressBar`
  (`Widget.RemoveFromParent` (`self.ProgressBarWidgetBP`)))

(fn `ActivateKeypad`
  (`/Game/CustomContent/UGC2289475071/KJModMacroLibrary.HandleClientServerLogic`
    (:`ServerLogic`
      (`self.PlayToolSoundFromServer`)
      (`/Game/CustomContent/UGC2289475071/Blueprints/Keypad/Keypad.KeypadActivated` (`self.Keypad`))
      (`self.HideProgressBar`))))

(fn `CreateAndShowToolsAssistinformation`
  (`self.ShowToolAssistUI`)
  (`self.SetToolAssistTitle` "Keypad Cracker" "Use on a keypad to activate what ever its connected to.")
  (`self.ClearToolAssistFunctions`)
  (bind _returnvalue (`self.CreateToolAssistFunction` "Start cracking keypad at crosshair."))
  (`self.SetToolAssistFunctionPrimaryDetails` _returnvalue "LeftMouse"))

(fn `UserConstructionScript`)