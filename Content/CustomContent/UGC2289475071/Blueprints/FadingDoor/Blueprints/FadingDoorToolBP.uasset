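; Fading Door tool that turns a prop the player aims at into a triggerable door.
; On click, the server line-traces from the camera, then spawns, attaches and tags a FadingDoorComponent actor, registers its trigger and records history.
; Trigger key, type and event name load from a save game and reload when the settings widget changes.
; Already-tagged props only reach a cast on attached actors, so updating is unfinished.
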(event `self.ReceiveBeginPlay`
  ;[0.9593 1 0.1335] BEGIN PLAY EVENT
  (`/Engine/EditorBlueprintResources/ActorMacros.Switch Has Authority`
    (:`Authority`
      ;;[1 1 1] Listen server?
      (bind _returnvalue (`KJModProxy.isDedicatedServer`))
      (if (not _returnvalue)
        (`|ExecutionSequence`
          (:`then_1`
            ;;[1 1 1] If local controlled; init once..
            (`self.IsLocalOrRemote` :!label _label
              (:`Local`
                (`KismetSystemLibrary.PrintString` "running on local")
                (`self.RegisterToolLocally`)
                (if (not (`self.Initialised`))
                  ;;[1 1 1] Reload settings
                  (`self.CreateAndShowToolsAssistInformation`)
                  (`self.InitSettings`)
                  (set `self.Initialised` true))))))))
    (:`Remote`
      (goto _label))))

(event `KJModToolProxyInterface.ToolProxy_PrimaryMouseClick`
  (params (pressed :type Boolean))
  ;[1 1 1] Primary Mouse Click - Triggers when player presses primary mouse button
  (if pressed
    (`self.MakeActorFadingDoor`) ; Look for actor to make fading door.
  ))

(event `MakeActorFadingDoor`
  (bind _triggerkey_key (break `InputChord` (`self.TriggerKey`)))
  ;[0.1274 0.6626 1] Make Actor into Fading Door - Looks for actor to convert into a fading door.
  (`/Engine/EditorBlueprintResources/ActorMacros.Switch Has Authority`
    (:`Authority`
      (if (`KismetInputLibrary.Key_IsValid` _triggerkey_key)
        (bind _returnvalue (`self.GetOwningPlayerProxy`))
        (bind _returnvalue_2 (`self.GetPawnRemoteCameraProxyComponent`))
        (bind _returnvalue_3 (`SceneComponent.K2_GetComponentLocation` _returnvalue_2))
        (bind (_outhit _returnvalue_4) (`KismetSystemLibrary.LineTraceSingleForObjects` :`Start` _returnvalue_3 :`End` (+ _returnvalue_3 (* (`SceneComponent.GetForwardVector` _returnvalue_2) 3500.0)) :`ObjectTypes` (`|MakeArray` "ObjectTypeQuery2" "ObjectTypeQuery4" :!type "EObjectTypeQuery Enum") :`DrawDebugType` "Persistent")) ; Line trace to see if player is looking at an actor
        (if _returnvalue_4
          (`self.PlayToolSoundEffect` "ToolSpawnSound")
          (if (`self.ActorHasTag` (`.HitActor` (`GameplayStatics.BreakHitResult` _outhit)) "Fading Door")
            ;;[1 1 1] Update Fading door on actor
            (for _array_element (`self.GetAttachedActors` (`.HitActor` (`GameplayStatics.BreakHitResult` _outhit)) true)
              (cast `/Game/CustomContent/UGC2289475071/Blueprints/FadingDoor/Blueprints/FadingDoorComponent` _array_element))
            (else
              ;;[1 1 1] Add fading door to actor
              (bind _returnvalue_5 (`|SpawnActorFromClass` "/Game/CustomContent/UGC2289475071/Blueprints/FadingDoor/Blueprints/FadingDoorComponent.FadingDoorComponent_C" (`KismetMathLibrary.Conv_VectorToTransform` (`self.K2_GetActorLocation` (`.HitActor` (`GameplayStatics.BreakHitResult` _outhit)))) "Undefined" "OverrideRootScale" null (`.HitActor` (`GameplayStatics.BreakHitResult` _outhit)) null))
              (`self.K2_AttachToActor` _returnvalue_5 (`.HitActor` (`GameplayStatics.BreakHitResult` _outhit)) "None" "SnapToTarget" "SnapToTarget" "SnapToTarget" true)
              (`self.RegisterTriggerActor` _returnvalue_5) ; replace with trigger actor function
              (`self.SetTrigger` _returnvalue_5 true (`self.TriggerType`) (`self.TriggerKey`) (`self.TriggerEventName`)) ; replace with trigger actor function
              (`KismetSystemLibrary.PrintString` "set trigger and registered actor")
              (`/Engine/EditorBlueprintResources/StandardMacros.IsValid` _returnvalue_5
                (:`Is Valid`
                  (`self.UpdateHistoryOwningClient` _returnvalue_5)
                  (`KismetArrayLibrary.Array_Add` (`Actor.Tags` (`.HitActor` (`GameplayStatics.BreakHitResult` _outhit))) "Fading Door")))))
          (else
            (`self.PlayToolSoundEffect` "ToolIllegalOpSound")))
        (else
          (`self.ShowMessageOnOwningClient` "Fading Door - No key specified!"))))))

(event `ShowMessageOnOwningClient`
  (params (Message :type String))
  ;[1 1 1] Show Message From Server - Does a show message on client from server side code.
  (`self.ShowMessage` Message 5.0 true null))

(event `UpdateHistoryOwningClient`
  (params (ObjectToAttach :type "Actor Object Reference"))
  ;[1 1 1] Update the history (to reflect last selection as most recent)
  (`self.AddHistoryEntry` (make `KJModToolHistoryItem` ObjectToAttach "Removing fading door" "Fading Door")))

(event `InitSettings`
  ;[1 1 1] Load settings
  (bind _returnvalue (`self.LoadToolSettings` "FadingDoorBaseSettings"))
  (`/Engine/EditorBlueprintResources/StandardMacros.IsValid` _returnvalue ; No save? use defaults
    (:`Is Valid`
      (bind _asbase_tool_save_game_bp (cast `/Game/CustomContent/UGC2289475071/Blueprints/BaseToolSaveGameBP` _returnvalue))
      (`self.RealiseSettings` (`/Game/CustomContent/UGC2289475071/Blueprints/BaseToolSaveGameBP.Triggerable` _asbase_tool_save_game_bp) (`/Game/CustomContent/UGC2289475071/Blueprints/BaseToolSaveGameBP.TriggerType` _asbase_tool_save_game_bp) (`/Game/CustomContent/UGC2289475071/Blueprints/BaseToolSaveGameBP.TriggerKey` _asbase_tool_save_game_bp) (`/Game/CustomContent/UGC2289475071/Blueprints/BaseToolSaveGameBP.TriggerEventName` _asbase_tool_save_game_bp)))))

(event `RealiseSettings`
  (params (Triggerable :type Boolean) (Selection :type Integer) (TriggerKey :type "InputChord Structure") (TriggerEventName :type String))
  ;[1 1 1] SERVER LOAD - These settings are used server side
  (`|ExecutionSequence`
    (:`then_1`
      (switch `int` Selection
        (:`0`
          (set `self.TriggerType` "KeyHeldTrigger") ; replace with fkjmod trigger type
        )
        (:`1`
          (set `self.TriggerType` "KeyPressToggle") ; replace with fkjmod trigger type
        )
        (:`2`
          (set `self.TriggerType` "NamedEventToggleTrigger") ; replace with fkjmod trigger type
        )))
    (:`then_2`
      (set `self.TriggerKey` TriggerKey))
    (:`then_3`
      (set `self.TriggerEventName` TriggerEventName))))

(event `TriggerWidgetSettingsChanged`
  ;[1 1 1] TriggerWidgetSettingsChanged - Run from the trigger settings widget
  (`self.InitSettings`))

(fn `CreateAndShowToolsAssistInformation`
  (`self.ShowToolAssistUI`)
  (`self.SetToolAssistTitle` "Fading Door" "Makes it so that a prop can be used as a door.")
  (`self.ClearToolAssistFunctions`)
  (bind _returnvalue (`self.CreateToolAssistFunction` "Add/Update fading door functionality to Prop"))
  (`self.SetToolAssistFunctionPrimaryDetails` _returnvalue "LeftMouse"))

(fn `ToolProxy_GetToolSettingPanel`
  (returns (ReturnValue :type "Widget Object Reference"))
  (`/Engine/EditorBlueprintResources/StandardMacros.IsValid` (`self.ToolSettingsWidget`)
    (:`Is Valid`
      _)
    (:`Is Not Valid`
      (bind _returnvalue (`|CreateWidget` "/Game/CustomContent/UGC2289475071/Blueprints/FadingDoor/Blueprints/UI/FadingDoorSettingsWidgetBP.FadingDoorSettingsWidgetBP_C" (`GameplayStatics.GetPlayerController` 0) self))
      (`/Game/CustomContent/UGC2289475071/Blueprints/FadingDoor/Blueprints/UI/FadingDoorSettingsWidgetBP.CreatedEvent` _returnvalue)
      (bind _output_get (set `self.ToolSettingsWidget` _returnvalue))
      ;[1 1 1] We want to listen to changes from the trigger widget part
      (add `/Game/CustomContent/UGC2289475071/Blueprints/TriggerWidgetBP.TriggerWidgetUpdated` (`/Game/CustomContent/UGC2289475071/Blueprints/FadingDoor/Blueprints/UI/FadingDoorSettingsWidgetBP.FadingDoorTriggerWidgetBP` _output_get) (`|CreateDelegate` :!event `TriggerWidgetSettingsChanged`))))
  (return (`self.ToolSettingsWidget`)))

(fn `UserConstructionScript`)