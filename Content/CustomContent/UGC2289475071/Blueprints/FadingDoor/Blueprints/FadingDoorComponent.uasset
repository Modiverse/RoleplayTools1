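; Fading door helper that makes a target Door actor passable and swaps it to an opacity material while activated.
; On BeginPlay the server snapshots each primitive component's collision mode, physics state and materials into a struct.
; Activated disables collision and swaps materials, while Deactivated and Destroyed restore both from the snapshot.
; Changes go through multicast events, skipping material swaps on dedicated servers; the physics flag is passed but never applied.
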(event `self.ReceiveBeginPlay`
  ;[1 1 1] Begin Play - Creates and saves the door struct.
  (`/Engine/EditorBlueprintResources/ActorMacros.Switch Has Authority`
    (:`Authority`
      (bind _fadingdoorstruct (`self.MakeFadingDoorStruct` (`self.Door`)))
      (set `self.FadingDoorStruct` _fadingdoorstruct))))

(event `self.ReceiveDestroyed`
  (bind (_fadingdoorstruct_actor _fadingdoorstruct_primitivecomponents) (break `/Game/CustomContent/UGC2289475071/Blueprints/FadingDoor/Blueprints/FadingDoorStruct` (`self.FadingDoorStruct`)))
  ;[1 1 1] Destroyed - Fading door was removed so we reset the actor.
  (for _array_element _fadingdoorstruct_primitivecomponents
    (`self.ChangePhyscisAndCollisionMulticast` (break `/Game/CustomContent/UGC2289475071/Blueprints/FadingDoor/Blueprints/FadingDoorComponentStruct` _array_element) (`.CollisionMode_8_A71209C14F94B222B8BB2C9E439F8731` (break `/Game/CustomContent/UGC2289475071/Blueprints/FadingDoor/Blueprints/FadingDoorComponentStruct` _array_element)) (`.Physics_15_3635973748483DC1BBD5FF8CFD38AD45` (break `/Game/CustomContent/UGC2289475071/Blueprints/FadingDoor/Blueprints/FadingDoorComponentStruct` _array_element)))
    (for _array_element_2 (`.Materials_16_499611C4487C69D8F22E0AAB7F50C1B3` (break `/Game/CustomContent/UGC2289475071/Blueprints/FadingDoor/Blueprints/FadingDoorComponentStruct` _array_element))
      (`self.ChangeMaterialOnClient` (break `/Game/CustomContent/UGC2289475071/Blueprints/FadingDoor/Blueprints/FadingDoorComponentStruct` _array_element) (break `/Game/CustomContent/UGC2289475071/Blueprints/FadingDoor/Blueprints/FadingDoorComponentMaterialStruct` _array_element_2) (`.MaterialElementIndex_7_3AA3DA4D435C036DADD5BAA31E2370FC` (break `/Game/CustomContent/UGC2289475071/Blueprints/FadingDoor/Blueprints/FadingDoorComponentMaterialStruct` _array_element_2))))))

(event `KJModTriggerInterface.Activated`
  (bind (_fadingdoorstruct_actor _fadingdoorstruct_primitivecomponents) (break `/Game/CustomContent/UGC2289475071/Blueprints/FadingDoor/Blueprints/FadingDoorStruct` (`self.FadingDoorStruct`)))
  ;[1 1 1] Activated - Fading door was activated
  (for _array_element _fadingdoorstruct_primitivecomponents
    (`self.ChangePhyscisAndCollisionMulticast` (break `/Game/CustomContent/UGC2289475071/Blueprints/FadingDoor/Blueprints/FadingDoorComponentStruct` _array_element))
    (for _array_element_2 (`.Materials_16_499611C4487C69D8F22E0AAB7F50C1B3` (break `/Game/CustomContent/UGC2289475071/Blueprints/FadingDoor/Blueprints/FadingDoorComponentStruct` _array_element))
      (`self.ChangeMaterialOnClient` (break `/Game/CustomContent/UGC2289475071/Blueprints/FadingDoor/Blueprints/FadingDoorComponentStruct` _array_element) "/Game/CustomContent/UGC2289475071/Blueprints/FadingDoor/Materials/FadingDoorOpacityMaterial.FadingDoorOpacityMaterial" (`.MaterialElementIndex_7_3AA3DA4D435C036DADD5BAA31E2370FC` (break `/Game/CustomContent/UGC2289475071/Blueprints/FadingDoor/Blueprints/FadingDoorComponentMaterialStruct` _array_element_2))))))

(event `KJModTriggerInterface.Deactivated`
  (bind (_fadingdoorstruct_actor _fadingdoorstruct_primitivecomponents) (break `/Game/CustomContent/UGC2289475071/Blueprints/FadingDoor/Blueprints/FadingDoorStruct` (`self.FadingDoorStruct`)))
  ;[1 1 1] Deactivated - Fading door was deactivated
  (for _array_element _fadingdoorstruct_primitivecomponents
    (`self.ChangePhyscisAndCollisionMulticast` (break `/Game/CustomContent/UGC2289475071/Blueprints/FadingDoor/Blueprints/FadingDoorComponentStruct` _array_element) (`.CollisionMode_8_A71209C14F94B222B8BB2C9E439F8731` (break `/Game/CustomContent/UGC2289475071/Blueprints/FadingDoor/Blueprints/FadingDoorComponentStruct` _array_element)) (`.Physics_15_3635973748483DC1BBD5FF8CFD38AD45` (break `/Game/CustomContent/UGC2289475071/Blueprints/FadingDoor/Blueprints/FadingDoorComponentStruct` _array_element)))
    (for _array_element_2 (`.Materials_16_499611C4487C69D8F22E0AAB7F50C1B3` (break `/Game/CustomContent/UGC2289475071/Blueprints/FadingDoor/Blueprints/FadingDoorComponentStruct` _array_element))
      (`self.ChangeMaterialOnClient` (break `/Game/CustomContent/UGC2289475071/Blueprints/FadingDoor/Blueprints/FadingDoorComponentStruct` _array_element) (break `/Game/CustomContent/UGC2289475071/Blueprints/FadingDoor/Blueprints/FadingDoorComponentMaterialStruct` _array_element_2) (`.MaterialElementIndex_7_3AA3DA4D435C036DADD5BAA31E2370FC` (break `/Game/CustomContent/UGC2289475071/Blueprints/FadingDoor/Blueprints/FadingDoorComponentMaterialStruct` _array_element_2))))))

(event `ChangeMaterialOnClient`
  (params (Component :type "PrimitiveComponent Object Reference") (Material :type "MaterialInterface Object Reference") (MaterialIndex :type Integer))
  ;[1 1 1] ChangeMaterialOnClient - Multicast event that sets a certain material on a component.
  (`/Engine/EditorBlueprintResources/ActorMacros.Switch Has Authority`
    (:`Authority`
      ;;[1 1 1] Listen server?
      (if (not (`KismetSystemLibrary.IsDedicatedServer`))
        (`PrimitiveComponent.SetMaterial` Component MaterialIndex Material :!label _label)))
    (:`Remote`
      (goto _label))))

(event `ChangePhyscisAndCollisionMulticast`
  (params (Component :type "PrimitiveComponent Object Reference") (Collision :type "ECollisionEnabled Enum" :default "NoCollision") (PhysicsEnabled :type Boolean))
  ;[1 1 1] Change PhysicsAndCollisionMulticast - Sets the given components physcis and collisions trhough a multicast.
  (`PrimitiveComponent.SetCollisionEnabled` Component Collision))

(fn `MakeFadingDoorComponentStruct`
  (params (DoorComponent :type "PrimitiveComponent Object Reference"))
  (returns (ComponentStruct :type "/Game/CustomContent/UGC2289475071/Blueprints/FadingDoor/Blueprints/FadingDoorComponentStruct Structure"))
  (locals (LocalMaterials :type "Array of /Game/CustomContent/UGC2289475071/Blueprints/FadingDoor/Blueprints/FadingDoorComponentMaterialStruct Structure"))
  (bind _returnvalue (`PrimitiveComponent.GetNumMaterials` DoorComponent))
  (`KismetSystemLibrary.PrintString` (`KismetStringLibrary.Concat_StrStr` "number of materials: " (`KismetStringLibrary.Conv_IntToString` _returnvalue)))
  (for _index (range (+ _returnvalue 1))
    (`KismetSystemLibrary.PrintString` (`KismetStringLibrary.Conv_IntToString` _index))
    (`KismetArrayLibrary.Array_Add` (`local.LocalMaterials`) (make `/Game/CustomContent/UGC2289475071/Blueprints/FadingDoor/Blueprints/FadingDoorComponentMaterialStruct` (`PrimitiveComponent.GetMaterial` DoorComponent _index) _index)))
  (return (make `/Game/CustomContent/UGC2289475071/Blueprints/FadingDoor/Blueprints/FadingDoorComponentStruct` DoorComponent (`PrimitiveComponent.GetCollisionEnabled` DoorComponent) (`SceneComponent.IsSimulatingPhysics` DoorComponent "None") (`local.LocalMaterials`))))

(fn `MakeFadingDoorStruct`
  (params (DoorActor :type "Actor Object Reference"))
  (returns (FadingDoorStruct :type "/Game/CustomContent/UGC2289475071/Blueprints/FadingDoor/Blueprints/FadingDoorStruct Structure"))
  (locals (LocalPrimitiveComponents :type "Array of /Game/CustomContent/UGC2289475071/Blueprints/FadingDoor/Blueprints/FadingDoorComponentStruct Structure"))
  (for _array_element (`self.K2_GetComponentsByClass` (`self.Door`) "/Script/Engine.PrimitiveComponent")
    (bind _componentstruct (`self.MakeFadingDoorComponentStruct` _array_element))
    (`KismetArrayLibrary.Array_Add` (`local.LocalPrimitiveComponents`) _componentstruct))
  (return (make `/Game/CustomContent/UGC2289475071/Blueprints/FadingDoor/Blueprints/FadingDoorStruct` DoorActor (`local.LocalPrimitiveComponents`))))

(fn `UserConstructionScript`)