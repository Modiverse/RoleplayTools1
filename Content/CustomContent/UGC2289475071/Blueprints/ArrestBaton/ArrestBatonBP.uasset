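; Arrest baton tool for Civil Protection: primary click arrests the player in front, secondary click releases them.
; A short server-side camera line trace finds the target pawn, whose "Arrested" tag tracks its state.
; Arresting strips tools and weapons through the player's KJModPlayerProxy and teleports them to a random "Jail"-tagged actor; unarresting kills them as a placeholder for restoring gear.
; On BeginPlay, the local owner registers the tool and shows its assist UI.
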(event `self.ReceiveBeginPlay`
  ;[0.9593 1 0.1335] BEGIN PLAY EVENT
  (`/Engine/EditorBlueprintResources/ActorMacros.Switch Has Authority`
    (:`Authority`
      ;;[1 1 1] Listen server?
      (if (not (`KismetSystemLibrary.IsDedicatedServer`))
        (`|ExecutionSequence`
          (:`then_1`
            ;;[1 1 1] If local controlled; init once..
            (`self.IsLocallyControlled` :!label _label
              (:`Local`
                (`self.RegisterToolLocally`)
                (if (not (`self.Initialised`))
                  (set `self.Initialised` true)
                  (`self.Create and Show Tools Assist Information`) ; Create tool info widget
                )))))))
    (:`Remote`
      (goto _label))))

(event `KJModToolProxyInterface.ToolProxy_PrimaryMouseClick`
  (params (pressed :type Boolean))
  ;[1 1 1] Primary Mouse Click - Triggers when player presses primary mouse button
  (if pressed
    (`self.ArrestPlayer`) ; Runs arrest player function on server side.
  ))

(event `ArrestPlayer`
  ;[1 1 1] Arrest Player - Server side event for looking for player and arresting them.
  (`/Engine/EditorBlueprintResources/ActorMacros.Switch Has Authority`
    (:`Authority`
      (bind (_hit _playerpawn) (`self.LookForPlayer`)) ; Check if a player is in front of the player
      (if _hit
        (if (not (`self.ActorHasTag` _playerpawn "Arrested"))
          (`KismetArrayLibrary.Array_Add` (`Actor.Tags` _playerpawn) "Arrested")
          (bind _aspawn (cast `Pawn` _playerpawn))
          (bind _outactors (`GameplayStatics.GetAllActorsOfClass` "/Script/KillerJimModProxy.KJModPlayerProxy"))
          (for _array_element _outactors
            (if (== (`KJModPlayerProxy.playerController` _array_element) (`Pawn.GetController` _aspawn))
              (`KJModPlayerProxy.StripTools` _array_element)
              (`KJModPlayerProxy.StripWeapons` _array_element)
              (`KJModPlayerProxy.ShowMessage` _array_element "You have been arrested!" 5 false null)
              (break)))
          (bind _outactors_2 (`GameplayStatics.GetAllActorsWithTag` "Jail")) ; Get all jail positions
          (`self.K2_SetActorLocation` _playerpawn (`self.K2_GetActorLocation` (`|GetArrayItem` _outactors_2 (`KismetMathLibrary.RandomInteger` (`KismetArrayLibrary.Array_Length` _outactors_2)))) false true) ; Move player to jail position
        )))))

(event `KJModToolProxyInterface.ToolProxy_SecondaryMouseClick`
  (params (pressed :type Boolean))
  ;[1 1 1] Secondary Mouse Click - Triggers when the player uses the secondary button
  (if pressed
    (`self.UnarrestPlayer`) ; Runs server side event for unarresting a player
  ))

(event `UnarrestPlayer`
  ;[1 1 1] Unarrest Player - Server side event for looking for player and unarresting them.
  (bind (_hit _playerpawn) (`self.LookForPlayer`)) ; Look for player infront of player
  (if _hit
    (if (`self.ActorHasTag` _playerpawn "Arrested")
      (`KismetArrayLibrary.Array_RemoveItem` (`Actor.Tags` _playerpawn) "Arrested")
      (bind _aspawn (cast `Pawn` _playerpawn))
      (bind _outactors (`GameplayStatics.GetAllActorsOfClass` "/Script/KillerJimModProxy.KJModPlayerProxy"))
      (for _array_element _outactors
        (if (== (`KJModPlayerProxy.playerController` _array_element) (`Pawn.GetController` _aspawn))
          (`KJModPlayerProxy.Kill` _array_element true) ; To be replaced with a "unstrip" function.
          (`KJModPlayerProxy.ShowMessage` _array_element "You have been unarrested!" 5 false null)
          (break))))))

(fn `Create and Show Tools Assist Information`
  ;[1 1 1] Create and Show Tools Assist Information - Shows the assist ui and updates the info
  (`self.ShowToolAssistUI`)
  (`self.SetToolAssistTitle` "Arrest Baton" "A tool used by Civil Protection to keep naughty players at bay.")
  (`self.ClearToolAssistFunctions`)
  (`|ExecutionSequence`
    (:`then_0`
      (bind _returnvalue (`self.CreateToolAssistFunction` "Arrest player"))
      (`self.SetToolAssistFunctionPrimaryDetails` _returnvalue "LeftMouse"))
    (:`then_1`
      (bind _returnvalue_2 (`self.CreateToolAssistFunction` "Unarrest player"))
      (`self.SetToolAssistFunctionPrimaryDetails` _returnvalue_2 "RightMouse"))))

(fn `LookForPlayer`
  (returns (Hit :type Boolean) (PlayerPawn :type "Actor Object Reference"))
  (`/Engine/EditorBlueprintResources/ActorMacros.Switch Has Authority`
    (:`Authority`
      (bind _returnvalue (`self.GetOwningPlayerProxy`))
      (bind _returnvalue_2 (`self.GetPawnRemoteCameraProxyComponent`))
      (bind _returnvalue_3 (`SceneComponent.K2_GetComponentLocation` _returnvalue_2))
      (bind _returnvalue_4 (`SceneComponent.GetForwardVector` _returnvalue_2))
      (bind (_outhit _returnvalue_5) (`KismetSystemLibrary.LineTraceSingleForObjects` (+ _returnvalue_3 (* _returnvalue_4 50.0)) (+ _returnvalue_3 (* _returnvalue_4 200.0)) (`|MakeArray` "ObjectTypeQuery3" :!type "EObjectTypeQuery Enum") false (`|MakeArray` (`KJModPlayerProxy.playerPawn` _returnvalue) :!type "Actor Object Reference") "Persistent")) ; Line trace to see if player is looking at an actor
      (return _returnvalue_5 (`.HitActor` (`GameplayStatics.BreakHitResult` _outhit))))))

(fn `UserConstructionScript`)