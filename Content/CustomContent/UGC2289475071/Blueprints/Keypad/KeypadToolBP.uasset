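; Keypad placement tool that lets a player spawn keypads, described in its UI as controlling other tool-spawned items.
; Each tick, the local client's camera trace positions a ghost keypad against the hit surface using the impact normal, mirroring the transform to the server.
; Primary click enables the ghost's collision via a multicast event, leaves it placed and requests a fresh server-spawned ghost, captured in the item-spawned callback.
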(event `self.ReceiveBeginPlay`
  ;[0.9593 1 0.1335] BEGIN PLAY EVENT
  (`/Game/CustomContent/UGC2289475071/KJModMacroLibrary.HandleClientServerLogic`
    (:`ClientLogic`
      ;;[1 1 1] If local controlled; init once..
      (`self.IsLocallyControlled`
        (:`Local`
          (`self.RegisterToolLocally`)
          (if (not (`self.Initialised`))
            ;;[1 1 1] Reload settings - TODO
            (`self.CreateAndShowToolsAssistinformation`)
            (set `self.Initialised` true)
            (`self.CreateGhostKeypad`)))))))

(event `self.ReceiveTick`
  (params (DeltaSeconds :type "Float (single-precision)"))
  (`/Game/CustomContent/UGC2289475071/KJModMacroLibrary.HandleClientServerLogic`
    (:`ClientLogic`
      (`self.IsLocallyControlled`
        (:`Local`
          (bind _returnvalue (`self.GetPawnCameraComponent`))
          (bind _returnvalue_2 (`SceneComponent.K2_GetComponentLocation` _returnvalue))
          (bind (_outhit _returnvalue_3) (`KismetSystemLibrary.LineTraceSingle` _returnvalue_2 (+ _returnvalue_2 (* (`SceneComponent.GetForwardVector` _returnvalue) 3500.0)) "TraceTypeQuery1" true (`|MakeArray` (`GameplayStatics.GetPlayerPawn` 0) :!type "Actor Object Reference")))
          (if _returnvalue_3
            (bind (_bblockinghit _binitialoverlap _time _distance _location _impactpoint _normal _impactnormal _physmat _hitactor) (`GameplayStatics.BreakHitResult` _outhit))
            (`/Engine/EditorBlueprintResources/StandardMacros.IsValid` _hitactor
              (:`Is Valid`
                (`/Engine/EditorBlueprintResources/StandardMacros.IsValid` (`self.GhostKeypad`) ; May not be replicated from server (yet)
                  (:`Is Valid`
                    (bind _rotation (`self.RotationFromImpactNormal` _impactpoint _impactnormal)
                      (:`Out`
                        (`self.SetKeypadInformationOwningClient` false _location _rotation)
                        (set `self.GhostKeypadVisible` true))))
                  (:`Is Not Valid`
                    (`self.SetKeypadInformationOwningClient` false :!label _label)
                    (set `self.GhostKeypadVisible` false))))
              (:`Is Not Valid`
                (goto _label)))
            (else
              (goto _label))))))))

(event `SetKeypadInformationOwningClient`
  (params (Visible :type Boolean) (Location :type "Vector Structure") (Rotation :type "Rotator Structure"))
  (bind _ghostkeypad (`self.GhostKeypad`))
  (`self.SetKeypadInformationServer` Visible Location Rotation)
  (`/Engine/EditorBlueprintResources/StandardMacros.IsValid` _ghostkeypad
    (:`Is Valid`
      (`self.K2_SetActorLocation` _ghostkeypad Location false true)
      (`self.K2_SetActorRotation` _ghostkeypad Rotation true)
      (`self.SetActorHiddenInGame` _ghostkeypad Visible))))

(event `SetKeypadInformationServer`
  (params (Visible :type Boolean) (Location :type "Vector Structure") (Rotation :type "Rotator Structure"))
  (bind _ghostkeypad (`self.GhostKeypad`))
  (`/Engine/EditorBlueprintResources/StandardMacros.IsValid` _ghostkeypad
    (:`Is Valid`
      (`self.K2_SetActorLocation` _ghostkeypad Location false true)
      (`self.K2_SetActorRotation` _ghostkeypad Rotation true)
      (`self.SetActorHiddenInGame` _ghostkeypad Visible))))

(event `KJModToolProxyInterface.ToolProxy_PrimaryMouseClick`
  (params (pressed :type Boolean))
  (if pressed
    (`/Engine/EditorBlueprintResources/StandardMacros.IsValid` (`self.GhostKeypad`)
      (:`Is Valid`
        (if (`self.GhostKeypadVisible`)
          (`self.KeypadCollisionMulticast`)
          (set `self.GhostKeypad` null)
          (`self.CreateGhostKeypad`))))))

(event `KeypadCollisionMulticast`
  (`PrimitiveComponent.SetCollisionEnabled` (`/Game/CustomContent/UGC2289475071/Blueprints/Keypad/Keypad.Cube` (`self.GhostKeypad`)) "QueryAndPhysics"))

(event `KJModToolProxyInterface.ToolProxy_ItemSpawned`
  (params (spawnedActor :type "Actor Object Reference"))
  ;[1 1 1] (interface) Item Spawned - From Pawn
  (bind _askeypad (cast `/Game/CustomContent/UGC2289475071/Blueprints/Keypad/Keypad` spawnedActor)
    (:`then`
      (`/Engine/EditorBlueprintResources/StandardMacros.IsValid` (`self.GhostKeypad`) ; First time? it's our "ghost" wheel
        (:`Is Valid`)
        (:`Is Not Valid`
          (set `self.GhostKeypad` _askeypad))))
    (:`CastFailed`
      (`parent.ToolProxy_ItemSpawned` spawnedActor) ; Probably a Q menu spawning; let parent deal with it
    )))

(fn `CreateAndShowToolsAssistinformation`
  (`self.ShowToolAssistUI`)
  (`self.SetToolAssistTitle` "Wheels" "A keypad that can be used to control other items spawned by tools.")
  (`self.ClearToolAssistFunctions`)
  (bind _returnvalue (`self.CreateToolAssistFunction` "Add a keypad to the desired spot."))
  (`self.SetToolAssistFunctionPrimaryDetails` _returnvalue "LeftMouse"))

(fn `CreateGhostKeypad`
  (bind _returnvalue (`GameplayStatics.GetPlayerCameraManager` 0))
  (`self.SpawnItem` "/Game/CustomContent/UGC2289475071/Blueprints/Keypad/Keypad" (+ (`self.K2_GetActorLocation` _returnvalue) (* (`self.GetActorForwardVector` _returnvalue) 500.0))) ; Spawns item on the server
)

(fn `UserConstructionScript`)