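; Keypad actor in a UGC mod that turns on blocking collision once spawned, with debug aids for network replication.
; The HasSpawned RepNotify sets the Root and Keypad components to BlockAllDynamic with query and physics, then prints a confirmation.
; Each tick, server logic multicasts the Keypad's world position to draw a short-lived debug sphere at the server-side location.
; No keypad input or interaction logic is present.
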(event `self.ReceiveTick`
  (params (DeltaSeconds :type "Float (single-precision)"))
  (`/Game/CustomContent/UGC2289475071/KJModMacroLibrary.HandleClientServerLogic`
    (:`ServerLogic`
      (`self.ShowServerPosMulticast` (`SceneComponent.K2_GetComponentLocation` (`self.Keypad`))))))

(event `ShowServerPosMulticast`
  (params (Pos :type "Vector Structure"))
  (`KismetSystemLibrary.DrawDebugSphere` Pos 10.0 12 (struct :`R` 1.0 :`G` 1.0 :`B` 1.0 :`A` 1.0) 0.1))

(fn `OnRep_HasSpawned`
  (bind _root (`self.Root`))
  (bind _keypad (`self.Keypad`))
  (`PrimitiveComponent.SetCollisionProfileName` _root "BlockAllDynamic" true)
  (`PrimitiveComponent.SetCollisionEnabled` _root "QueryAndPhysics")
  (`PrimitiveComponent.SetCollisionProfileName` _keypad "BlockAllDynamic" true)
  (`PrimitiveComponent.SetCollisionEnabled` _keypad "QueryAndPhysics")
  (`KJModProxy.PrintString_KJMod` self "Set collision on keypad." true true (struct) 5.0))

(fn `UserConstructionScript`)