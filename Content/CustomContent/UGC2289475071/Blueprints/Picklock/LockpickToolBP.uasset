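; Lockpick player tool that unlocks a door when primary click is held while aiming at it.
; The local client relays press state and calls a server-side camera line trace every tick to find actors implementing the door interface.
; A hit starts a five-second timer that calls UnlockDoor, while release or losing the door cancels it.
; A progress widget tracks the timer, and a tool-assist panel shows the control.
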(event `self.ReceiveBeginPlay`
  ;[0.9593 1 0.1335] BEGIN PLAY EVENT
  (`/Game/CustomContent/UGC2289475071/KJModMacroLibrary.HandleClientServerLogic`
    (:`ClientLogic`
      ;;[1 1 1] If local controlled; init once..
      (`self.IsLocallyControlled`
        (:`Local`
          (`self.RegisterToolLocally`)
          (`self.CreateAndShowToolsAssistinformation`)
          (bind _returnvalue (`|CreateWidget` "/Game/CustomContent/UGC2289475071/Blueprints/Picklock/LockpickProgressBarWidgetBP.LockpickProgressBarWidgetBP_C" (`GameplayStatics.GetPlayerController` 0)))
          (set `self.ProgressBarWidgetBP` _returnvalue))))))

(event `self.ReceiveTick`
  (params (DeltaSeconds :type "Float (single-precision)"))
  (bind _activatetimer (`self.ActivateTimer`))
  (bind _returnvalue (`KismetSystemLibrary.K2_GetTimerElapsedTimeHandle` _activatetimer))
  (`/Game/CustomContent/UGC2289475071/KJModMacroLibrary.HandleClientServerLogic`
    (:`ClientLogic`
      (`self.IsLocallyControlled`
        (:`Local`
          (`self.LookForLockToPicklockServer`)
          (if (`KismetSystemLibrary.K2_IsTimerActiveHandle` _activatetimer)
            (`/Game/CustomContent/UGC2289475071/Blueprints/Picklock/LockpickProgressBarWidgetBP.UpdateProgress` (`self.ProgressBarWidgetBP`) (/ _returnvalue (+ _returnvalue (`KismetSystemLibrary.K2_GetTimerRemainingTimeHandle` _activatetimer))))))))))

(event `LookForLockToPicklockServer`
  (bind _activatetimer (`self.ActivateTimer`))
  (bind _activatetimer_2 (`self.ActivateTimer`))
  (`/Game/CustomContent/UGC2289475071/KJModMacroLibrary.HandleClientServerLogic`
    (:`ServerLogic`
      (if (`self.Pressed`)
        (bind _returnvalue (`self.GetPawnRemoteCameraProxyComponent`))
        (bind _returnvalue_2 (`SceneComponent.K2_GetComponentLocation` _returnvalue))
        (bind (_outhit _returnvalue_3) (`KismetSystemLibrary.LineTraceSingle` _returnvalue_2 (+ _returnvalue_2 (* (`SceneComponent.GetForwardVector` _returnvalue) 500.0)) "TraceTypeQuery1" true (`|MakeArray` (`GameplayStatics.GetPlayerPawn` 0) :!type "Actor Object Reference"))) ; Look for keypad
        (if _returnvalue_3
          ;[1 1 1] CHeck if it implements door
          (if (`KismetSystemLibrary.DoesImplementInterface` (`.HitActor` (`GameplayStatics.BreakHitResult` _outhit)) "/Game/CustomContent/UGC2275057327/Doors/Interfaces/KJMod_VRP_Door_Interface.KJMod_VRP_Door_Interface_C")
            (`KismetSystemLibrary.PrintString` "found door")
            (if (not (`KismetSystemLibrary.K2_IsTimerActiveHandle` (`self.ActivateTimer`)))
              (set `self.Door` (`.HitActor` (`GameplayStatics.BreakHitResult` _outhit)))
              (bind _returnvalue_4 (`KismetSystemLibrary.K2_SetTimer` null "UnlockDoor" 5.0))
              (set `self.ActivateTimer` _returnvalue_4)
              (`self.ShowProgressBar`))
            (else
              (`KismetSystemLibrary.PrintString` "didnt find door")
              (if (`KismetSystemLibrary.K2_IsValidTimerHandle` _activatetimer) :!label _label
                (`KismetSystemLibrary.K2_ClearAndInvalidateTimerHandle` _activatetimer)
                (`self.HideProgressBar`))))
          (else
            (goto _label)))
        (elif (`KismetSystemLibrary.K2_IsValidTimerHandle` _activatetimer_2)
          (`KismetSystemLibrary.K2_ClearAndInvalidateTimerHandle` _activatetimer_2)
          (`self.HideProgressBar`))))))

(event `KJModToolProxyInterface.ToolProxy_PrimaryMouseClick`
  (params (pressed :type Boolean))
  (`/Game/CustomContent/UGC2289475071/KJModMacroLibrary.HandleClientServerLogic`
    (:`ClientLogic`
      (`self.IsLocallyControlled`
        (:`Local`
          (`self.ToggledPressedOnServer` pressed))))))

(event `ToggledPressedOnServer`
  (params (Pressed :type Boolean))
  (set `self.Pressed` Pressed))

(event `PlayToolSoundFromServer`
  (`self.PlayToolSoundEffect` "ToolSpawnSound"))

(event `ShowProgressBar`
  (`UserWidget.AddToViewport` (`self.ProgressBarWidgetBP`) 0))

(event `HideProgressBar`
  (`Widget.RemoveFromParent` (`self.ProgressBarWidgetBP`)))

(fn `CreateAndShowToolsAssistinformation`
  (`self.ShowToolAssistUI`)
  (`self.SetToolAssistTitle` "Lockpick" "Use on a door to unlock it.")
  (`self.ClearToolAssistFunctions`)
  (bind _returnvalue (`self.CreateToolAssistFunction` "Start lock picking the door in front of you."))
  (`self.SetToolAssistFunctionPrimaryDetails` _returnvalue "LeftMouse"))

(fn `UnlockDoor`
  (`/Game/CustomContent/UGC2289475071/KJModMacroLibrary.HandleClientServerLogic`
    (:`ServerLogic`
      (`self.PlayToolSoundFromServer`)
      (`KismetSystemLibrary.PrintString` "unlocked door")
      ;[1 1 1] Unlock door
      (message `/Game/CustomContent/UGC2275057327/Doors/Interfaces/KJMod_VRP_Door_Interface.SetDoorLocked` (`self.Door`) false)
      (`self.HideProgressBar`))))

(fn `UserConstructionScript`)