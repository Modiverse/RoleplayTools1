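; Pocket tool that lets a player temporarily store up to four "Pocketable" actors and drop them again, last in first out.
; Primary click runs a server-side camera trace and attaches the hit actor to PocketPosition; secondary click detaches it in front of the camera.
; Each item records its primitives' physics and collision state, applied through a multicast because collision changes don't replicate correctly.
; Destroying the tool drops all pocketed items.
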(event `ShowMessageToLocalPlayer`
  (params (String :type String))
  ;[1 1 1] Show Message to Local Player - Run from server side to run message on owning client.
  (`self.ShowMessage` String 5.0 true))

(event `self.ReceiveDestroyed`
  ;[1 1 1] Destroyed Event - Runs when tools is destroyed.
  (`/Engine/EditorBlueprintResources/ActorMacros.Switch Has Authority`
    (:`Authority`
      ;;[1 1 1] Loop through all pocketed items and drop them on the floor.
      (for _ (`self.PocketedItems`)
        (`self.DropEntity`)))))

(event `self.ReceiveBeginPlay`
  ;[0.9593 1 0.1335] BEGIN PLAY EVENT
  (`/Engine/EditorBlueprintResources/ActorMacros.Switch Has Authority`
    (:`Authority`
      ;;[1 1 1] Listen server?
      (if (not (`KismetSystemLibrary.IsDedicatedServer`))
        (`|ExecutionSequence`)))
    (:`Remote`)))

(event `KJModToolProxyInterface.ToolProxy_PrimaryMouseClick`
  (params (pressed :type Boolean))
  ;[1 1 1] Primary Mouse Click - Triggers when the player uses the primary button
  (if pressed
    (`self.PickUpEntity`) ; Try to pick up something on the server.
  ))

(event `PickUpEntity`
  ;[1 1 1] PickUpEntity - Server side event for picking up a Actor.
  (`/Engine/EditorBlueprintResources/ActorMacros.Switch Has Authority`
    (:`Authority`
      (if (< (`KismetArrayLibrary.Array_Length` (`self.PocketedItems`)) 4)
        (bind _returnvalue (`self.GetOwningPlayerProxy`))
        (bind _returnvalue_2 (`self.GetPawnRemoteCameraProxyComponent`))
        (bind _returnvalue_3 (`SceneComponent.K2_GetComponentLocation` _returnvalue_2))
        (bind (_outhit _returnvalue_4) (`KismetSystemLibrary.LineTraceSingleForObjects` _returnvalue_3 (+ _returnvalue_3 (* (`SceneComponent.GetForwardVector` _returnvalue_2) 200.0)) (`|MakeArray` "ObjectTypeQuery2" "ObjectTypeQuery4" :!type "EObjectTypeQuery Enum") false (`|MakeArray` (`KJModPlayerProxy.playerPawn` _returnvalue) :!type "Actor Object Reference") "Persistent")) ; Line trace to see if player is looking at an actor
        (if _returnvalue_4
          (if (`self.ActorHasTag` (`.HitActor` (`GameplayStatics.BreakHitResult` _outhit)) "Pocketable")
            (bind _pocketitemstruct (`self.MakePocketItem` (`.HitActor` (`GameplayStatics.BreakHitResult` _outhit)))) ; Make pocket item from struct
            (`KismetArrayLibrary.Array_Add` (`self.PocketedItems`) _pocketitemstruct) ; Add struct to pocketed items
            (bind (_actor _primitivecomponents) (break `/Game/CustomContent/UGC2289475071/Blueprints/Pocket/PocketItemStruct` _pocketitemstruct))
            (`self.K2_AttachToComponent` _actor (`self.PocketPosition`) "None" "KeepRelative" "KeepRelative" "KeepRelative" true)
            (`self.SetActorScale3D` _actor (1.0 1.0 1.0))
            (`self.K2_SetActorLocation` _actor (`SceneComponent.K2_GetComponentLocation` (`self.PocketPosition`)) false false) ; Position the pocketed item at the pocket position
            ;;[1 1 1] Loop through all primitives and set it to not simulate physics and disable collision.
            (for _array_element _primitivecomponents
              (`self.UpdateComponentInformation` _array_element) ; Set Collision Enabled does not replicate correctl, therefore we need this.
            )))
        (else
          (`self.ShowMessageToLocalPlayer` "Your pocket is full."))))))

(event `KJModToolProxyInterface.ToolProxy_SecondaryMouseClick`
  (params (pressed :type Boolean))
  ;[1 1 1] Secondary Mouse Click - Triggers when the player uses the secondary button
  (if pressed
    (`self.DropEntity`) ; Run Drop Entity event on server
  ))

(event `DropEntity`
  (bind _returnvalue (- (`KismetArrayLibrary.Array_Length` (`self.PocketedItems`)) 1))
  (bind (_output_actor _output_primitivecomponents) (break `/Game/CustomContent/UGC2289475071/Blueprints/Pocket/PocketItemStruct` (`|GetArrayItem` (`self.PocketedItems`) _returnvalue)))
  ;[1 1 1] DropEntity - Server side event for dropping the last added entity from pocket.
  (`/Engine/EditorBlueprintResources/ActorMacros.Switch Has Authority`
    (:`Authority`
      (if (>= _returnvalue 0)
        (`self.K2_DetachFromActor` _output_actor "KeepWorld" "KeepWorld" "KeepWorld")
        (`self.SetActorScale3D` _output_actor (1.0 1.0 1.0))
        (bind _returnvalue_2 (`self.GetPawnRemoteCameraProxyComponent`))
        (`self.K2_SetActorLocation` _output_actor (+ (`SceneComponent.K2_GetComponentLocation` _returnvalue_2) (* (`SceneComponent.GetForwardVector` _returnvalue_2) (* (.y (`.BoxExtent` (`self.GetActorBounds` _output_actor false false))) 3.0))) false true)
        ;;[1 1 1] Loop through all primitive components and set simulate physics and collision to how it was pre pocketing.
        (for _array_element _output_primitivecomponents
          (`self.UpdateComponentInformation` _array_element) ; Set Collision Enabled does not replicate correctl, therefore we need this.
        )
        (`KismetArrayLibrary.Array_Remove` (`self.PocketedItems`) _returnvalue)
        (else
          (`self.ShowMessageToLocalPlayer` "Your pocket is empty!"))))))

(event `UpdateComponentInformation`
  (params (ItemComponent :type "/Game/CustomContent/UGC2289475071/Blueprints/Pocket/PocketItemComponentStruct Structure"))
  ;[1 1 1] Update Component Information - Updates the physics and collision settings for components in a multicast.
  (`PrimitiveComponent.SetSimulatePhysics` ItemComponent_Component_2_250A511B494CEE2F713DDBA18CD4AE85 ItemComponent_SimulatePhysics_5_9146D82146068BA44CE3378D19336C04)
  (`PrimitiveComponent.SetCollisionEnabled` ItemComponent_Component_2_250A511B494CEE2F713DDBA18CD4AE85 ItemComponent_CollisionMode_8_A71209C14F94B222B8BB2C9E439F8731))

(fn `Create and Show Tools Assist Information`
  ;[1 1 1] Create and Show Tools Assist Information - Shows the assist ui and updates the info
  (`self.ShowToolAssistUI`)
  (`self.SetToolAssistTitle` "Pocket" "A tool used for temporary storing of items.")
  (`self.ClearToolAssistFunctions`)
  (`|ExecutionSequence`
    (:`then_0`
      (bind _returnvalue (`self.CreateToolAssistFunction` "Add item to pocket"))
      (`self.SetToolAssistFunctionPrimaryDetails` _returnvalue "LeftMouse"))
    (:`then_1`
      (bind _returnvalue_2 (`self.CreateToolAssistFunction` "Remove item from pocket"))
      (`self.SetToolAssistFunctionPrimaryDetails` _returnvalue_2 "RightMouse"))))

(fn `MakePocketItem`
  (params (Item :type "Actor Object Reference"))
  (returns (PocketItemStruct :type "/Game/CustomContent/UGC2289475071/Blueprints/Pocket/PocketItemStruct Structure"))
  (locals (LocalComponentArray :type "Array of /Game/CustomContent/UGC2289475071/Blueprints/Pocket/PocketItemComponentStruct Structure"))
  (for _array_element (`self.K2_GetComponentsByClass` Item "/Script/Engine.PrimitiveComponent")
    (`KismetArrayLibrary.Array_Add` (`local.LocalComponentArray`) (make `/Game/CustomContent/UGC2289475071/Blueprints/Pocket/PocketItemComponentStruct` _array_element (`SceneComponent.IsSimulatingPhysics` _array_element "None") (`PrimitiveComponent.GetCollisionEnabled` _array_element))))
  (return (make `/Game/CustomContent/UGC2289475071/Blueprints/Pocket/PocketItemStruct` Item (`local.LocalComponentArray`))))

(fn `UserConstructionScript`
  (`parent.UserConstructionScript`))